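; Base enemy Blueprint that walks toward the level's end point and can be killed by damage.
; On BeginPlay, AndarAteOFim gets all BP_Final actors and issues an AIMoveTo toward each in a loop.
; AnyDamage subtracts the damage from Vida (health), then verificarvida destroys the actor once health reaches zero or below.
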(event Custom|Andar%20ate%20o%20fim
  ;[1 1 1] Andar ate o ponto final
  (bind _outactors (Actor|GetAllActorsOfClass "/Game/Programacao/BP_Final.BP_Final_C"))
  (for _array_element _outactors
    (AI|AIMoveTo self "0, 0, 0" _array_element 5.0 false)))

(event Custom|verificar%20vida
  (if (<= (Variables|Default|GetVida) 0.0)
    (Actor|DestroyActor)))

(event EventBeginPlay
  (CallFunction|AndarAteOFim))

(event Game|Damage|EventAnyDamage
  (params (Damage :type Float%20%28single-precision%29) (DamageType :type Damage%20Type%20Object%20Reference) (InstigatedBy :type Controller%20Object%20Reference) (DamageCauser :type Actor%20Object%20Reference))
  (Variables|Default|SetVida (- (Variables|Default|GetVida) Damage))
  (CallFunction|VerificarVida))

(fn ConstructionScript)